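; HuaweiVRCameraFoveated is a Huawei VR player rig with left and right motion controller components.
; On begin play it sets a floor tracking origin and activates the touch interface.
; Every tick it copies each HVR controller's position and orientation onto the matching component's relative transform.
; Gamepad Special Left teleports it to a hardcoded location and rotation; no foveation logic appears in the graphs.
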(event EventBeginPlay
  (Class|HeadMountedDisplayFunctionLibrary|SetTrackingOrigin "Floor")
  (Class|PlayerController|ActivateTouchInterface (Game|GetPlayerController 0)))

(event EventTick
  (params (DeltaSeconds :type Float%20%28single-precision%29))
  (Utilities|FlowControl|Sequence
    (:then_0
      (bind (_orientation _position) (Class|HVRControllerFunctionLibrary|GetHVRControllerOrientationandPosition "Right"))
      (Transformation|SetRelativeLocationAndRotation (Variables|Default|GetHVRMotionControllerR) _position _orientation false false))
    (:then_1
      (bind (_orientation_2 _position_2) (Class|HVRControllerFunctionLibrary|GetHVRControllerOrientationandPosition "Left"))
      (Transformation|SetRelativeLocationAndRotation (Variables|Default|GetHVRMotionControllerL) _position_2 _orientation_2 false false))))

(event Input|GamepadEvents|GamepadSpecialLeft
  (params (Key :type Key%20Structure :default "None"))
  (:Pressed
    (Transformation|Teleport "1000.000000,100.000000,1000.000000" "0.000000,75.000000, 0")))

(fn ConstructionScript)